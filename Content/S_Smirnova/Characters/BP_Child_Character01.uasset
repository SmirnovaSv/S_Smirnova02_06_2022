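; BP_Child_Character01 is a player-controlled character Blueprint that handles movement, look, jump and sprint input.
; Axis inputs move it along its forward and right vectors and feed controller yaw and pitch.
; Holding Sprint doubles the CharacterMovement walk speed, and releasing restores it.
; The Interact input only prints press and release messages, and BeginPlay and the construction script just call their parent versions.
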(event EventBeginPlay
  (|CallParentFunction))

(event Input|ActionEvents|InputActionInteract
  (params (Key :type Key%20Structure))
  ;[0.1832 1 0.1289] Входные данные
  (:Pressed
    (Development|PrintString "Press"))
  (:Released
    (Development|PrintString "Release")))

(event Input|ActionEvents|InputActionSprint
  (params (Key :type Key%20Structure))
  ;[0.1832 1 0.1289] Входные данные
  (:Pressed
    (Variables|/Script/Engine.CharacterMovementComponent|SetMaxWalkSpeed (Variables|Character|GetCharacterMovement) 9e+02))
  (:Released
    (Variables|/Script/Engine.CharacterMovementComponent|SetMaxWalkSpeed (Variables|Character|GetCharacterMovement) 4.5e+02)))

(event Input|ActionEvents|InputActionJump
  (params (Key :type Key%20Structure))
  ;[0.1832 1 0.1289] Входные данные
  (:Pressed
    (Character|Jump)))

(event Input|AxisEvents|InputAxisMoveRight
  (params (AxisValue :type Float%20%28single-precision%29))
  ;[0.1832 1 0.1289] Входные данные
  ;;[1 1 1] Перемещение
  (Pawn|Input|AddMovementInput (Transformation|GetActorRightVector) AxisValue false))

(event Input|AxisEvents|InputAxisMoveForward
  (params (AxisValue :type Float%20%28single-precision%29))
  ;[0.1832 1 0.1289] Входные данные
  ;;[1 1 1] Перемещение
  (Pawn|Input|AddMovementInput (Transformation|GetActorForwardVector) AxisValue false))

(event Input|AxisEvents|InputAxisTurn
  (params (AxisValue :type Float%20%28single-precision%29))
  ;[0.1832 1 0.1289] Входные данные
  ;;[1 1 1] Поворот
  (Pawn|Input|AddControllerYawInput AxisValue))

(event Input|AxisEvents|InputAxisLookUp
  (params (AxisValue :type Float%20%28single-precision%29))
  ;[0.1832 1 0.1289] Входные данные
  ;;[1 1 1] Поворот
  (Pawn|Input|AddControllerPitchInput AxisValue))

(fn ConstructionScript
  (|CallParentFunction))